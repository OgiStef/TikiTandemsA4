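; Player controller for the arena test mode that spawns the player's fighter and routes combat input to it.
; On BeginPlay it asks GM_ArenaTest to spawn and possess a BP_Magicman on the Red team, caches the pawn as BP_Tiki, then adds the combat mapping context.
; Enhanced Input events forward look, move and jump to that pawn.
; Basic, special and heavy attacks only print debug strings.
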(event `self.ReceiveBeginPlay`
  ;[0.1458 0.1458 0.1458] BeginPlay
  (bind _asgm_arena_test (cast `/Game/Core/Blueprints/Gamemodes/GM_ArenaTest` (`GameplayStatics.GetGameMode`)))
  (`/Game/Core/Blueprints/Gamemodes/GM_ArenaTest.SpawnAndPossessPlayer` _asgm_arena_test self "/Game/Core/Blueprints/Characters/Magicman/BP_Magicman.BP_Magicman_C" "Red" "None")
  (bind _asbp_tiki (cast `/Game/Core/Blueprints/TikiCharacter/Blueprint/BP_Tiki` (`self.K2_GetPawn`)))
  (set `self.BP_TikiReference` _asbp_tiki)
  (`/Game/Core/Blueprints/Functions/BFL_General.AddInputMappingContext` self "/Game/Core/Blueprints/Input/InputActionMappings/IMC_Combat.IMC_Combat"))

(event `EnhancedInput|/Game/Core/Blueprints/Input/InputActions/IA_Look`
  (params (ActionValue :type "Vector2D Structure") (ElapsedSeconds :type "Float (double-precision)") (TriggeredSeconds :type "Float (double-precision)") (InputAction :type "InputAction Object Reference" :default "/Game/Core/Blueprints/Input/InputActions/IA_Look.IA_Look"))
  ;[0.2344 0.2344 0.2344] BasicInput
  (:`Triggered`
    (`/Game/Core/Blueprints/TikiCharacter/Blueprint/BP_Tiki.LookInput` (`self.BP_TikiReference`) ActionValue_X ActionValue_Y)))

(event `EnhancedInput|/Game/Core/Blueprints/Input/InputActions/IA_BasicAttack`
  (params (ActionValue :type Boolean) (ElapsedSeconds :type "Float (double-precision)") (TriggeredSeconds :type "Float (double-precision)") (InputAction :type "InputAction Object Reference" :default "/Game/Core/Blueprints/Input/InputActions/IA_BasicAttack.IA_BasicAttack"))
  ;[0.3542 0.3542 0.3542] CombatInput
  (:`Triggered`
    (`KismetSystemLibrary.PrintString` "Basic")))

(event `EnhancedInput|/Game/Core/Blueprints/Input/InputActions/IA_Move`
  (params (ActionValue :type "Vector2D Structure") (ElapsedSeconds :type "Float (double-precision)") (TriggeredSeconds :type "Float (double-precision)") (InputAction :type "InputAction Object Reference" :default "/Game/Core/Blueprints/Input/InputActions/IA_Move.IA_Move"))
  ;[0.2344 0.2344 0.2344] BasicInput
  (:`Triggered`
    (`/Game/Core/Blueprints/TikiCharacter/Blueprint/BP_Tiki.MoveInput` (`self.BP_TikiReference`) ActionValue_X ActionValue_Y)))

(event `EnhancedInput|/Game/Core/Blueprints/Input/InputActions/IA_SpecialAttack`
  (params (ActionValue :type Boolean) (ElapsedSeconds :type "Float (double-precision)") (TriggeredSeconds :type "Float (double-precision)") (InputAction :type "InputAction Object Reference" :default "/Game/Core/Blueprints/Input/InputActions/IA_SpecialAttack.IA_SpecialAttack"))
  ;[0.3542 0.3542 0.3542] CombatInput
  (:`Triggered`
    (`KismetSystemLibrary.PrintString` "Speacial")))

(event `EnhancedInput|/Game/Core/Blueprints/Input/InputActions/IA_Jump`
  (params (ActionValue :type Boolean) (ElapsedSeconds :type "Float (double-precision)") (TriggeredSeconds :type "Float (double-precision)") (InputAction :type "InputAction Object Reference" :default "/Game/Core/Blueprints/Input/InputActions/IA_Jump.IA_Jump"))
  ;[0.2344 0.2344 0.2344] BasicInput
  (:`Started`
    (`/Game/Core/Blueprints/TikiCharacter/Blueprint/BP_Tiki.JumpInput` (`self.BP_TikiReference`))))

(event `EnhancedInput|/Game/Core/Blueprints/Input/InputActions/IA_HeavyAttack`
  (params (ActionValue :type Boolean) (ElapsedSeconds :type "Float (double-precision)") (TriggeredSeconds :type "Float (double-precision)") (InputAction :type "InputAction Object Reference" :default "/Game/Core/Blueprints/Input/InputActions/IA_HeavyAttack.IA_HeavyAttack"))
  ;[0.3542 0.3542 0.3542] CombatInput
  (:`Triggered`
    (`KismetSystemLibrary.PrintString` "Heavy")))

(fn `UserConstructionScript`)